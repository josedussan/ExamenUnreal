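; BP_Key is a collectible key pickup that the third-person character gathers by walking into its box trigger.
; On overlap it increments CollectedKeys on BP_ThirdPersonGameMode, prints the running total on screen in Spanish, and destroys itself.
; Each key also resets that game mode counter to zero on BeginPlay.
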(event OnComponentBeginOverlap(Box)
  (params (OverlappedComponent :type Primitive%20Component%20Object%20Reference) (OtherActor :type Actor%20Object%20Reference) (OtherComp :type Primitive%20Component%20Object%20Reference) (OtherBodyIndex :type Integer) (bFromSweep :type Boolean) (SweepResult :type Hit%20Result%20Structure%20%28by%20ref%29))
  (Utilities|Casting|CastToBP_ThirdPersonCharacter OtherActor)
  (bind _asbp_third_person_game_mode (Utilities|Casting|CastToBP_ThirdPersonGameMode (Game|GetGameMode)))
  (bind _output_get (Variables|/Game/ThirdPerson/Blueprints/BP_ThirdPersonGameMode.BP_ThirdPersonGameMode_C|SetCollectedKeys _asbp_third_person_game_mode (+ (Variables|/Game/ThirdPerson/Blueprints/BP_ThirdPersonGameMode.BP_ThirdPersonGameMode_C|GetCollectedKeys _asbp_third_person_game_mode) 1)))
  (Development|PrintString (Utilities|String|Append (Utilities|String|ToString(Text) (Utilities|Text|MakeLiteralText "Llaves recogidas: ")) (Utilities|String|ToString(Text) (Utilities|Text|MakeLiteralText (Utilities|Text|ToText(Integer) _output_get)))))
  (Actor|DestroyActor))

(event EventBeginPlay
  (bind _asbp_third_person_game_mode (Utilities|Casting|CastToBP_ThirdPersonGameMode (Game|GetGameMode)))
  (Variables|/Game/ThirdPerson/Blueprints/BP_ThirdPersonGameMode.BP_ThirdPersonGameMode_C|SetCollectedKeys _asbp_third_person_game_mode 0))

(event Collision|EventActorBeginOverlap
  (params (OtherActor :type Actor%20Object%20Reference)))

(event EventTick
  (params (DeltaSeconds :type Float%20%28single-precision%29)))

(fn ConstructionScript)