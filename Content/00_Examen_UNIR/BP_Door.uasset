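; BP_Door is a double sliding door whose two mesh panels part along their local X axis.
; BeginPlay caches each panel's starting relative location as the closed position.
; The OpenDoor event takes a boolean that plays or reverses a Timeline, which lerps the panels outward in opposite directions to open or back to close.
; The file has no active trigger of its own, as the overlap and Tick events are empty.
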(event Custom|OpenDoor
  (params (estado :type Boolean))
  (if estado
    (bind _newtrack_0 (Timeline|Timeline Play)
      (:Update
        (Transformation|SetRelativeLocation (Variables|Default|GetSM_door_Right) (Math|Vector|Lerp(Vector) (Variables|Default|GetposIniRight) (+ (Variables|Default|GetposIniRight) "80.000000,0.000000,0.000000") _newtrack_0) false false)
        (Transformation|SetRelativeLocation (Variables|Default|GetSM_door_Left) (Math|Vector|Lerp(Vector) (Variables|Default|GetposIniLeft) (+ (Variables|Default|GetposIniLeft) "-80.000000,0.000000,0.000000") _newtrack_0) false false)))
    (else
      (Timeline|Timeline Reverse))))

(event EventBeginPlay
  (Variables|Default|SetposIniRight (Variables|/Script/Engine.SceneComponent|GetRelativeLocation (Variables|Default|GetSM_door_Right)))
  (Variables|Default|SetposIniLeft (Variables|/Script/Engine.SceneComponent|GetRelativeLocation (Variables|Default|GetSM_door_Left))))

(event Collision|EventActorBeginOverlap
  (params (OtherActor :type Actor%20Object%20Reference)))

(event EventTick
  (params (DeltaSeconds :type Float%20%28single-precision%29)))

(fn ConstructionScript)