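; BP_FloorButton is a floor switch that opens and closes its linked Door.
; Its Box overlap enables and disables input while the third-person character stands on it.
; Pressing E toggles the button when the GameMode's CollectedKeys equals the Door's RequiredKeys, calling OpenDoor and swapping the hieroglyph mesh between red and green materials.
; Otherwise it prints how many keys are missing.
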(event OnComponentBeginOverlap(Box)
  (params (OverlappedComponent :type Primitive%20Component%20Object%20Reference) (OtherActor :type Actor%20Object%20Reference) (OtherComp :type Primitive%20Component%20Object%20Reference) (OtherBodyIndex :type Integer) (bFromSweep :type Boolean) (SweepResult :type Hit%20Result%20Structure%20%28by%20ref%29))
  (Utilities|Casting|CastToBP_ThirdPersonCharacter OtherActor)
  (Input|EnableInput (Game|GetPlayerController 0)))

(event OnComponentEndOverlap(Box)
  (params (OverlappedComponent :type Primitive%20Component%20Object%20Reference) (OtherActor :type Actor%20Object%20Reference) (OtherComp :type Primitive%20Component%20Object%20Reference) (OtherBodyIndex :type Integer))
  (Utilities|Casting|CastToBP_ThirdPersonCharacter OtherActor)
  (Input|DisableInput (Game|GetPlayerController 0)))

(event EventBeginPlay
  (Rendering|Material|SetMaterial (Variables|Default|GetSM_hieroglyph_007) 0 "/Game/00_Examen_UNIR/M_Rojo.M_Rojo"))

(event Collision|EventActorBeginOverlap
  (params (OtherActor :type Actor%20Object%20Reference)))

(event EventTick
  (params (DeltaSeconds :type Float%20%28single-precision%29)))

(event Input|KeyboardEvents|E
  (params (Key :type Key%20Structure :default "None"))
  (bind _door (Variables|Default|GetDoor))
  (bind _requiredkeys (Variables|/Game/00_Examen_UNIR/BP_Door.BP_Door_C|GetRequiredKeys _door))
  (:Pressed
    (bind _asbp_third_person_game_mode (Utilities|Casting|CastToBP_ThirdPersonGameMode (Game|GetGameMode)))
    (if (== (Variables|/Game/ThirdPerson/Blueprints/BP_ThirdPersonGameMode.BP_ThirdPersonGameMode_C|GetCollectedKeys _asbp_third_person_game_mode) _requiredkeys)
      (bind _output_get (Variables|Default|SetButtonActived (not (Variables|Default|GetButtonActived))))
      (if _output_get
        (Rendering|Material|SetMaterial (Variables|Default|GetSM_hieroglyph_007) 0 "/Game/00_Examen_UNIR/M_Verde.M_Verde")
        (Default|OpenDoor (Variables|Default|GetDoor) true)
        (else
          (Rendering|Material|SetMaterial (Variables|Default|GetSM_hieroglyph_007) 0 "/Game/00_Examen_UNIR/M_Rojo.M_Rojo")
          (Default|OpenDoor (Variables|Default|GetDoor) false)))
      (else
        (Development|PrintString (Utilities|String|Append (Utilities|String|ToString(Text) (Utilities|Text|MakeLiteralText "Te faltan llaves: ")) (Utilities|String|ToString(Text) (Utilities|Text|MakeLiteralText (Utilities|Text|ToText(Integer) (- _requiredkeys (Variables|/Game/ThirdPerson/Blueprints/BP_ThirdPersonGameMode.BP_ThirdPersonGameMode_C|GetCollectedKeys _asbp_third_person_game_mode)))))))))))

(fn ConstructionScript)